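; BP_Player is a player Blueprint that moves a ball with physics and triggers a left flipper.
; Horizontal and Vertical axis inputs share one AddImpulse call on the Sphere, pushing it in the XY plane by axis value scaled by Speed.
; Pressing InteractFire prints a debug "Hello" and sends InteractMessage to FlipperLeft through an always-true branch.
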(event `InputAxis|Horizontal`
  (params (AxisValue :type "Float (single-precision)"))
  ;[1 1 1] Move A Ball
  (`PrimitiveComponent.AddImpulse` (`self.Sphere`) (* (`KismetMathLibrary.MakeVector` (stale `InputAxis|Vertical` AxisValue) AxisValue) (`self.Speed`)) "None" false :!label _label))

(event `InputAxis|Vertical`
  (params (AxisValue :type "Float (single-precision)"))
  ;[1 1 1] Move A Ball
  (goto _label))

(event `InputAction|InteractFire`
  (params (Key :type "Key Structure"))
  (:`Pressed`
    (`KismetSystemLibrary.PrintString` "Hello")
    (if true
      (message `/Game/Blueprints/InteractionInterface.Interact` (`.FlipperLeft` (`self.FlipperLeft`)) null))))

(fn `UserConstructionScript`)