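; StarterButton_Blueprint is a pinball starter button that launches the ball resting against it.
; A mesh hit sets a touching flag, stores the actor as the ball if it casts to Pinball_Blueprint, and prints a debug message.
; The HitBall event, with no caller in this file, applies the hit's normal impulse scaled by BumpPower and clamped in size as a velocity change, then clears the flag.
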(event `self.StaticMeshComponent.OnComponentHit`
  (params (HitComponent :type "PrimitiveComponent Object Reference") (OtherActor :type "Actor Object Reference") (OtherComp :type "PrimitiveComponent Object Reference") (NormalImpulse :type "Vector Structure") (Hit :type "HitResult Structure (by ref)"))
  (set `self.TouchingStarterButton` true)
  (bind _aspinball_blueprint (cast `/Game/Blueprints/Pinball_Blueprint` OtherActor))
  (set `self.BallRef` _aspinball_blueprint)
  (`KismetSystemLibrary.PrintString` "Toching"))

(event `HitBall`
  (if (`self.TouchingStarterButton`)
    (`PrimitiveComponent.AddImpulse` (`StaticMeshActor.StaticMeshComponent` (`self.BallRef`)) (`KismetMathLibrary.ClampVectorSize` (* (stale `self.StaticMeshComponent.OnComponentHit` NormalImpulse) (`KismetMathLibrary.Conv_IntToDouble` (`self.BumpPower`))) 4001.0 5000.0) "None" true)
    (set `self.TouchingStarterButton` false)))

(fn `UserConstructionScript`)