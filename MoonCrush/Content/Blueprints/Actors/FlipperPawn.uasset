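; Player pawn for pinball-style controls, driving a left and right flipper and triggering the ball starter.
; Input sets pressed flags, and Tick uses RInterpTo to swing each flipper between rest and raised yaw at FlipperSpeed.
; Releasing clears an EndReached flag, so even a short tap completes the full swing before the flipper returns.
; The starter input casts StarterButtonRef to StarterButton_Blueprint and calls HitBall.
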(event `self.ReceiveTick`
  (params (DeltaSeconds :type "Float (single-precision)"))
  (bind _left (`self.Left`))
  (bind _right (`self.Right`))
  (bind (_relativerotation_roll _relativerotation_pitch _relativerotation_yaw) (`KismetMathLibrary.BreakRotator` (`SceneComponent.RelativeRotation` _right)))
  (bind (_relativerotation_roll_2 _relativerotation_pitch_2 _relativerotation_yaw_2) (`KismetMathLibrary.BreakRotator` (`SceneComponent.RelativeRotation` _left)))
  (`|ExecutionSequence`
    (:`then_0`
      ;[1 1 1] Flipper as Pawn
      (if (`self.LeftFlipperEndReached`)
        (if (`self.LeftFlipperPressed`)
          (`SceneComponent.K2_SetRelativeRotation` _left (`KismetMathLibrary.RInterpTo` (`SceneComponent.RelativeRotation` (`self.Left`)) (struct :`Yaw` 80.0) DeltaSeconds (`self.FlipperSpeed`)) false false :!label _label)
          ;;[1 1 1] Comment
          (if (`KismetMathLibrary.NearlyEqual_FloatFloat` _relativerotation_yaw_2 80.0 1.0)
            (set `self.LeftFlipperEndReached` true))
          (else
            (`SceneComponent.K2_SetRelativeRotation` (`self.Left`) (`KismetMathLibrary.RInterpTo` (`SceneComponent.RelativeRotation` (`self.Left`)) (struct :`Yaw` 140.0) DeltaSeconds (`self.FlipperSpeed`)) false false)))
        (else
          (goto _label))))
    (:`then_1`
      ;[1 1 1] Flipper as Pawn
      (if (`self.RightFlipperEndReached`)
        (if (`self.RightFlipperPressed`)
          (`SceneComponent.K2_SetRelativeRotation` _right (`KismetMathLibrary.RInterpTo` (`SceneComponent.RelativeRotation` (`self.Right`)) (struct :`Yaw` 280.0) DeltaSeconds (`self.FlipperSpeed`)) false false :!label _label_2)
          (if (`KismetMathLibrary.NearlyEqual_FloatFloat` _relativerotation_yaw -80.0 1.0)
            (set `self.RightFlipperEndReached` true))
          (else
            (`SceneComponent.K2_SetRelativeRotation` (`self.Right`) (`KismetMathLibrary.RInterpTo` (`SceneComponent.RelativeRotation` (`self.Right`)) (struct :`Yaw` 220.0) DeltaSeconds (`self.FlipperSpeed`)) false false)))
        (else
          (goto _label_2))))))

(event `InputAction|InteractLeftFlipper`
  (params (Key :type "Key Structure"))
  ;[1 1 1] Flipper as Pawn
  (:`Pressed`
    (set `self.LeftFlipperPressed` true))
  (:`Released`
    (set `self.LeftFlipperPressed` false)
    (set `self.LeftFlipperEndReached` false)))

(event `InputAction|InteractRightFlipper`
  (params (Key :type "Key Structure"))
  ;[1 1 1] Flipper as Pawn
  (:`Pressed`
    (set `self.RightFlipperPressed` true))
  (:`Released`
    (set `self.RightFlipperPressed` false)
    (set `self.RightFlipperEndReached` false)))

(event `InputAction|InteractStarterButton`
  (params (Key :type "Key Structure"))
  (:`Pressed`
    (bind _asstarter_button_blueprint (cast `/Game/Blueprints/Actors/StarterButton_Blueprint` (`self.StarterButtonRef`))
      (:`then`
        (`/Game/Blueprints/Actors/StarterButton_Blueprint.HitBall` _asstarter_button_blueprint))
      (:`CastFailed`
        (`KismetSystemLibrary.PrintString` "Hello")))))

(fn `UserConstructionScript`)