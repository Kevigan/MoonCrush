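; Pinball bumper actor that kicks the ball and awards score when struck.
; On a hit from Pinball_Blueprint, it applies the amplified, clamped normal impulse as a velocity change to both its own mesh and the ball's.
; It then calls BumperHit and adds HitScore through MyGameMode.
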(event `self.StaticMeshComponent.OnComponentHit`
  (params (HitComponent :type "PrimitiveComponent Object Reference") (OtherActor :type "Actor Object Reference") (OtherComp :type "PrimitiveComponent Object Reference") (NormalImpulse :type "Vector Structure") (Hit :type "HitResult Structure (by ref)"))
  (bind _aspinball_blueprint (cast `/Game/Blueprints/Pinball_Blueprint` OtherActor))
  (`PrimitiveComponent.AddImpulse` (`self.StaticMeshComponent`) (`KismetMathLibrary.ClampVectorSize` (* NormalImpulse 5.0) 1.0 5000.0) "None" true)
  (`PrimitiveComponent.AddImpulse` (`StaticMeshActor.StaticMeshComponent` _aspinball_blueprint) (`KismetMathLibrary.ClampVectorSize` (* NormalImpulse 5.0) 1.0 5000.0) "None" true)
  (`self.BumperHit`)
  (bind _asmy_game_mode (cast `/Game/Blueprints/MyGameMode` (`GameplayStatics.GetGameMode`)))
  (`/Game/Blueprints/MyGameMode.AddScore` _asmy_game_mode (`self.HitScore`)))

(fn `UserConstructionScript`)